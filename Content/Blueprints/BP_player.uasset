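; BP_player is a Paper2D player character for a platformer, driven by flipbook animation.
; BeginPlay adds the IMC_PLATFORM Enhanced Input mapping context.
; Each Tick, UpdateAnimation picks run or idle on the ground, and rise or fall in the air from velocity.
; The jump and move input events are empty, their movement nodes are disconnected, and NewFunction is an uncalled run/idle switch.
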(event Input|EnhancedActionEvents|EnhancedInputActionIA_JUMP
  (params (ActionValue :type Boolean) (ElapsedSeconds :type Float%20%28double-precision%29) (TriggeredSeconds :type Float%20%28double-precision%29) (InputAction :type Input%20Action%20Object%20Reference :default "/Game/input/actions/IA_JUMP.IA_JUMP")))

(event Input|EnhancedActionEvents|EnhancedInputActionIA_MOVE
  (params (ActionValue :type Float%20%28double-precision%29) (ElapsedSeconds :type Float%20%28double-precision%29) (TriggeredSeconds :type Float%20%28double-precision%29) (InputAction :type Input%20Action%20Object%20Reference :default "/Game/input/actions/IA_MOVE.IA_MOVE")))

(event EventBeginPlay
  (bind _asplayer_controller (Utilities|Casting|CastToPlayerController (Pawn|GetController)))
  (Input|AddMappingContext (PlayerController|LocalPlayerSubsystems|GetEnhancedInputLocalPlayerSubsystem _asplayer_controller) "/Game/input/IMC_PLATFORM.IMC_PLATFORM" 0 "(bIgnoreAllPressedKeysUntilRelease=True,bForceImmediately=False,bNotifyUserSettings=False)"))

(event Collision|EventActorBeginOverlap
  (params (OtherActor :type Actor%20Object%20Reference)))

(event EventTick
  (params (DeltaSeconds :type Float%20%28single-precision%29))
  (CallFunction|UpdateAnimation))

(fn ConstructionScript)

(fn NewFunction
  (params (Condition :type Boolean))
  (if Condition
    (Sprite|SetFlipbook (Variables|Default|GetSprite) "/Game/paper_ssests/Character/Flipbook/FP_RUN.FP_RUN")
    (else
      (Sprite|SetFlipbook (Variables|Default|GetSprite) "/Game/paper_ssests/Character/Flipbook/FP_PLAYER_IDOL.FP_PLAYER_IDOL"))))

(fn UpdateAnimation
  (if (AI|Components|NavMovement|IsMovingonGround (Variables|Character|GetCharacterMovement))
    (if (> (Math|Vector|VectorLength (Transformation|GetVelocity)) 0.0)
      (Sprite|SetFlipbook (Variables|Default|GetSprite) "/Game/paper_ssests/Character/Flipbook/FP_RUN.FP_RUN")
      (else
        (Sprite|SetFlipbook (Variables|Default|GetSprite) "/Game/paper_ssests/Character/Flipbook/FP_PLAYER_IDOL.FP_PLAYER_IDOL")))
    (elif (< (.z (Transformation|GetVelocity)) -1e+02)
      (Sprite|SetFlipbook (Variables|Default|GetSprite) "/Game/paper_ssests/Character/Flipbook/FP_FALL.FP_FALL")
      (else
        (Sprite|SetFlipbook (Variables|Default|GetSprite) "/Game/paper_ssests/Character/Flipbook/FP_RISE.FP_RISE")))))